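; MetaplexTerminal is a terminal actor that registers itself with a nearby player for Metaplex machine interaction.
; Trigger overlaps cast the other actor to SolanaPlayerController, setting or clearing its IsNearMetaplexMachine flag and NearbyTerminal reference.
; An AIPerception binding hides the TextRender when the updated-actor list is empty.
; BeginPlay also holds a character-cast check that briefly shows the text, then hides it after a delay.
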(event `self.ReceiveBeginPlay`
  (bind _textrender (`self.TextRender`))
  (add `AIPerceptionComponent.OnPerceptionUpdated` (`self.AIPerception`) (delegate `OnPerceptionUpdated_Event`))
  (cast `/Game/ThirdPerson/Blueprints/BP_ThirdPersonCharacter` (`|GetArrayItem` (stale `OnPerceptionUpdated_Event` UpdatedActors)))
  (`SceneComponent.SetVisibility` _textrender true false)
  (`KismetSystemLibrary.Delay` 5.0)
  (`SceneComponent.SetVisibility` _textrender false false))

(event `OnPerceptionUpdated_Event`
  (params (UpdatedActors :type "Array of Actor Object Reference (by ref)"))
  (if (not (!= (`KismetArrayLibrary.Array_Length` UpdatedActors) 0))
    (`SceneComponent.SetVisibility` (`self.TextRender`) false false)))

(event `self.ReceiveTick`
  (params (DeltaSeconds :type "Float (single-precision)")))

(event `self.Trigger.OnComponentBeginOverlap`
  (params (OverlappedComponent :type "PrimitiveComponent Object Reference") (OtherActor :type "Actor Object Reference") (OtherComp :type "PrimitiveComponent Object Reference") (OtherBodyIndex :type Integer) (bFromSweep :type Boolean) (SweepResult :type "HitResult Structure (by ref)"))
  (bind _assolana_player_controller (cast `/SolanaSDK/ProgramIntegrationStore/blueprint/SolanaPlayerController` OtherActor))
  (set `/SolanaSDK/ProgramIntegrationStore/blueprint/SolanaPlayerController.isNearMetaplexMachine` true _assolana_player_controller)
  (set `/SolanaSDK/ProgramIntegrationStore/blueprint/SolanaPlayerController.NearbyTerminal` self _assolana_player_controller))

(event `self.Trigger.OnComponentEndOverlap`
  (params (OverlappedComponent :type "PrimitiveComponent Object Reference") (OtherActor :type "Actor Object Reference") (OtherComp :type "PrimitiveComponent Object Reference") (OtherBodyIndex :type Integer))
  (bind _assolana_player_controller (cast `/SolanaSDK/ProgramIntegrationStore/blueprint/SolanaPlayerController` OtherActor))
  (set `/SolanaSDK/ProgramIntegrationStore/blueprint/SolanaPlayerController.isNearMetaplexMachine` false _assolana_player_controller)
  (set `/SolanaSDK/ProgramIntegrationStore/blueprint/SolanaPlayerController.NearbyTerminal` null _assolana_player_controller))

(fn `UserConstructionScript`)