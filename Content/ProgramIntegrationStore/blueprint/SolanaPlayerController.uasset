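; Player controller that lets the player enter and leave a nearby Metaplex machine terminal with the E key.
; Entering blends the view to the terminal and focuses its login widget with the cursor shown; leaving restores the default character view and game-only input.
; Setter functions track terminal proximity and the default character.
; SendToTranquility triggers a link-stream sync that drops the transaction message and calls an empty function.
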(event `Key|E`
  (params (Key :type "Key Structure"))
  (bind _nearbyterminal (`self.NearbyTerminal`))
  (:`Pressed`
    (if (`self.isUsingMetaplexMachine`)
      (`self.PossessDefaultCharacter`)
      (set `self.isUsingMetaplexMachine` false)
      (`WidgetBlueprintLibrary.SetInputMode_GameOnly` self)
      (set `self.bShowMouseCursor` false)
      (elif (`self.isNearMetaplexMachine`)
        (`self.PossessTerminal` 1.0 _nearbyterminal)
        (set `self.isUsingMetaplexMachine` true)
        (set `self.bShowMouseCursor` true)
        (`WidgetBlueprintLibrary.SetInputMode_GameAndUIEx` self (`WidgetComponent.GetWidget` (`/SolanaSDK/ProgramIntegrationStore/blueprint/MetaplexTerminal.loginscreen` _nearbyterminal)) "DoNotLock" false)))))

(event `ConnectToLinkStream`
  (params (TransactionMessage :type String))
  (`self.SyncToLinkStream` ""))

(fn `PossessDefaultCharacter`
  (`self.SetViewTargetWithBlend` (`self.DefaultCharcter`)))

(fn `PossessTerminal`
  (params (BlendTime :type "Float (single-precision)") (NewViewTarget :type "Actor Object Reference"))
  (`self.SetViewTargetWithBlend` NewViewTarget BlendTime))

(fn `SendToTranquility`
  (params (TransactionMessage :type String))
  (`self.ConnectToLinkStream` TransactionMessage))

(fn `SetDefaultCharacter`
  (params (DefaultPossess :type "/Game/ThirdPerson/Blueprints/BP_ThirdPersonCharacter Object Reference"))
  (set `self.DefaultCharcter` DefaultPossess))

(fn `SetTCPcomponent`
  (params (TCp :type "Object Object Reference")))

(fn `SolanaPlayerController_AutoGenFunc`
  (params (ConnectionId :type Integer)))

(fn `SyncToLinkStream`
  (params (Message :type String)))

(fn `UpdateTerminalState`
  (params (State :type Boolean) (Terminal :type "/SolanaSDK/ProgramIntegrationStore/blueprint/MetaplexTerminal Object Reference"))
  (set `self.isNearMetaplexMachine` State)
  (set `self.NearbyTerminal` Terminal))

(fn `UserConstructionScript`)