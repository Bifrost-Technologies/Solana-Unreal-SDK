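; Trigger button Blueprint that switches a target light and calls an interact program event when activated.
; Begin and end overlap on its collision both feed one FlipFlop, alternating between on and off.
; The on branch turns the button green, lights the target and fires the program call, while off only restores red and turns the light off.
; The Construction Script creates the button's dynamic material instance.
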(event `self.Trigger collision.OnComponentBeginOverlap`
  (params (OverlappedComponent :type "PrimitiveComponent Object Reference") (OtherActor :type "Actor Object Reference") (OtherComp :type "PrimitiveComponent Object Reference") (OtherBodyIndex :type Integer) (bFromSweep :type Boolean) (SweepResult :type "HitResult Structure (by ref)"))
  (bind _button_light_material (`self.Button light material`))
  (bind _target_light (`self.Target light`))
  (`/Engine/EditorBlueprintResources/StandardMacros.FlipFlop` :!label _label
    (:`A`
      (`MaterialInstanceDynamic.SetScalarParameterValue` _button_light_material "State" 1.0) ; Change a scalar value in the button material that turns it green
      (`/SolanaSDK/ExampleContent/Blueprint_Communication/Blueprints/BP_Light_Bulb_Basic.Toggle light` _target_light true) ; Call a custom event in the target Blueprint to turn its light on
      (`self.InteractProgramEvent`))
    (:`B`
      (`MaterialInstanceDynamic.SetScalarParameterValue` _button_light_material "State" 0.0) ; Change a scalar value in the button material that turns it back to red
      (`/SolanaSDK/ExampleContent/Blueprint_Communication/Blueprints/BP_Light_Bulb_Basic.Toggle light` _target_light false) ; Turn the light off
    )))

(event `self.Trigger collision.OnComponentEndOverlap`
  (params (OverlappedComponent :type "PrimitiveComponent Object Reference") (OtherActor :type "Actor Object Reference") (OtherComp :type "PrimitiveComponent Object Reference") (OtherBodyIndex :type Integer))
  (goto _label))

(fn `UserConstructionScript`
  (bind _returnvalue (`PrimitiveComponent.CreateDynamicMaterialInstance` (`self.ButtonMesh`) 1 null "None"))
  (set `self.Button light material` _returnvalue) ; Save a reference to the Dynamic Material Instance for use in the event graph
)