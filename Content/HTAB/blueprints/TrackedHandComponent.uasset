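; Actor component that gives a VR pawn tracked hands with optional laser pointers.
; On BeginPlay it spawns a TrackedHand actor if the owner has MotionController components, then applies UE4 or Oculus skeleton meshes per HandSkeletonType.
; It attaches each hand mesh to a controller by matching "left" in the MotionSource name, treating others as right.
; It finally sets per-hand laser visibility and scales both beams from BeamLength.
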(event `InitAndSpawnHands`
  (bind _returnvalue (`self.GetOwner`))
  ;[1 1 1] Init and Spawn Hands
  (if (!= (`KismetArrayLibrary.Array_Length` (`Actor.K2_GetComponentsByClass` _returnvalue "/Script/HeadMountedDisplay.MotionControllerComponent")) 0)
    (bind _returnvalue_2 (`|SpawnActorFromClass` "/Game/HTAB/blueprints/TrackedHand.TrackedHand_C" (`SceneComponent.K2_GetComponentToWorld` (`Actor.RootComponent` _returnvalue)) "Undefined" "OverrideRootScale" _returnvalue (`self.Hand Skeleton Type`) null))
    (set `self.thisTrackedHand` _returnvalue_2)))

(event `self.ReceiveBeginPlay`
  (bind _thistrackedhand (`self.thisTrackedHand`))
  (bind _thistrackedhand_2 (`self.thisTrackedHand`))
  (bind _thistrackedhand_3 (`self.thisTrackedHand`))
  (bind _thistrackedhand_4 (`self.thisTrackedHand`))
  (bind _thistrackedhand_5 (`self.thisTrackedHand`))
  (bind _returnvalue (`Actor.K2_GetComponentsByClass` (`self.GetOwner`) "/Script/HeadMountedDisplay.MotionControllerComponent"))
  (bind _laserpointer_r (`/Game/HTAB/blueprints/TrackedHand.LaserPointer_R` _thistrackedhand))
  (bind _laserpointer_l (`/Game/HTAB/blueprints/TrackedHand.LaserPointer_L` _thistrackedhand_4))
  (bind _laserpointer_l_2 (`/Game/HTAB/blueprints/TrackedHand.LaserPointer_L` _thistrackedhand_3))
  (bind _laserpointer_r_2 (`/Game/HTAB/blueprints/TrackedHand.LaserPointer_R` _thistrackedhand_3))
  (bind _oculushand_r_oc (`/Game/HTAB/blueprints/TrackedHand.OculusHand_R_Oc` (`self.thisTrackedHand`)))
  (bind _oculushand_l_oc (`/Game/HTAB/blueprints/TrackedHand.OculusHand_L_Oc` (`self.thisTrackedHand`)))
  (bind _oculushand_r_ue4 (`/Game/HTAB/blueprints/TrackedHand.OculusHand_R_UE4` (`self.thisTrackedHand`)))
  (bind _oculushand_l_ue4 (`/Game/HTAB/blueprints/TrackedHand.OculusHand_L_UE4` (`self.thisTrackedHand`)))
  (bind (_relativescale3d_x _relativescale3d_y) (`KismetMathLibrary.BreakVector` (`SceneComponent.RelativeScale3D` _laserpointer_r_2)))
  (bind (_relativescale3d_x_2 _relativescale3d_y_2) (`KismetMathLibrary.BreakVector` (`SceneComponent.RelativeScale3D` _laserpointer_l_2)))
  (`|ExecutionSequence`
    (:`then_0`
      (`self.InitAndSpawnHands`))
    (:`then_1`
      ;[0.3695 1 0.9202] Spawn Default Hand Mesh of either Oculus or Unreal Skeleton
      (switch `/Game/HTAB/meshes/HandSkeleton_Type` (`self.Hand Skeleton Type`)
        (:`NewEnumerator0`
          (if (`KismetSystemLibrary.IsValid` (`self.RightHandMesh_UE4`))
            (`SkinnedMeshComponent.SetSkinnedAssetAndUpdate` _oculushand_r_ue4 (`self.RightHandMesh_UE4`) true)
            (`SceneComponent.SetHiddenInGame` _oculushand_r_ue4 false false)
            (else
              (`self.Deactivate` _oculushand_r_ue4)))
          (if (`KismetSystemLibrary.IsValid` (`self.LeftHandMesh_UE4`))
            (`SkinnedMeshComponent.SetSkinnedAssetAndUpdate` _oculushand_l_ue4 (`self.LeftHandMesh_UE4`) true)
            (`SceneComponent.SetHiddenInGame` _oculushand_l_ue4 false false)
            (else
              (`self.Deactivate` _oculushand_l_ue4))))
        (:`NewEnumerator1`
          (if (`KismetSystemLibrary.IsValid` (`self.RightHandMesh_Oc`))
            (`SkinnedMeshComponent.SetSkinnedAssetAndUpdate` _oculushand_r_oc (`self.RightHandMesh_Oc`) true)
            (`SceneComponent.SetHiddenInGame` _oculushand_r_oc false false)
            (else
              (`self.Deactivate` _oculushand_r_oc)))
          (if (`KismetSystemLibrary.IsValid` (`self.LeftHandMesh_Oc`))
            (`SkinnedMeshComponent.SetSkinnedAssetAndUpdate` _oculushand_l_oc (`self.LeftHandMesh_Oc`) true)
            (`SceneComponent.SetHiddenInGame` _oculushand_l_oc false false)
            (else
              (`self.Deactivate` _oculushand_l_oc))))))
    (:`then_2`
      (if (!= (`KismetArrayLibrary.Array_Length` _returnvalue) 0)
        (for _array_element _returnvalue
          (switch `/Game/HTAB/meshes/HandSkeleton_Type` (`self.Hand Skeleton Type`)
            (:`NewEnumerator0`
              (bind _returnvalue_2 (`KismetStringLibrary.Contains` (`KismetStringLibrary.Conv_NameToString` (`MotionControllerComponent.MotionSource` _array_element)) "left"))
              (if _returnvalue_2
                (`SceneComponent.K2_AttachToComponent` (`/Game/HTAB/blueprints/TrackedHand.OculusHand_L_UE4` _thistrackedhand_5) _array_element "None" "SnapToTarget" "KeepRelative" "KeepWorld" true)
                (else
                  (`SceneComponent.K2_AttachToComponent` (`/Game/HTAB/blueprints/TrackedHand.OculusHand_R_UE4` _thistrackedhand_5) _array_element "None" "SnapToTarget" "SnapToTarget" "KeepWorld" true))))
            (:`NewEnumerator1`
              (if _returnvalue_2
                (`SceneComponent.K2_AttachToComponent` (`/Game/HTAB/blueprints/TrackedHand.OculusHand_L_Oc` _thistrackedhand_2) _array_element "None" "SnapToTarget" "SnapToTarget" "KeepWorld" true)
                (else
                  (`SceneComponent.K2_AttachToComponent` (`/Game/HTAB/blueprints/TrackedHand.OculusHand_R_Oc` _thistrackedhand_2) _array_element "None" "SnapToTarget" "SnapToTarget" "KeepWorld" true))))))
        (else
          (`KismetSystemLibrary.PrintString` "Error: No MotionControllers Detected, not a valid Pawn"))))
    (:`then_3`
      ;[1 1 1] Laser Pointers On/Off
      (if (`self.RightHandLaserOn`)
        (set `/Game/HTAB/blueprints/TrackedHand.isRLaserEnabled` true _thistrackedhand)
        (`SceneComponent.SetVisibility` _laserpointer_r true false)
        (else
          (set `/Game/HTAB/blueprints/TrackedHand.isRLaserEnabled` false _thistrackedhand)
          (`SceneComponent.SetVisibility` _laserpointer_r false false)))
      (if (`self.LeftHandLaserOn`)
        (set `/Game/HTAB/blueprints/TrackedHand.isLLaserEnabled` true _thistrackedhand_4)
        (`SceneComponent.SetVisibility` _laserpointer_l true false)
        (else
          (set `/Game/HTAB/blueprints/TrackedHand.isLLaserEnabled` false _thistrackedhand_4)
          (`SceneComponent.SetVisibility` _laserpointer_l false false))))
    (:`then_4`
      ;[1 1 1] Set Laser Beam Length
      (`SceneComponent.SetRelativeScale3D` _laserpointer_l_2 (`KismetMathLibrary.MakeVector` _relativescale3d_x_2 _relativescale3d_y_2 (`KismetMathLibrary.Conv_IntToDouble` (/ (`self.BeamLength`) 100))))
      (`SceneComponent.SetRelativeScale3D` _laserpointer_r_2 (`KismetMathLibrary.MakeVector` _relativescale3d_x _relativescale3d_y (`KismetMathLibrary.Conv_IntToDouble` (/ (`self.BeamLength`) 100)))))))