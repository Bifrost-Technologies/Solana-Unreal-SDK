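; Oculus hand-tracking actor with pinch-driven laser pointers and clicks, supporting either the UE4 or Oculus hand skeleton.
; Construction attaches tip colliders, lasers and widget interaction to the chosen skeleton, destroys the unused one, and builds per-bone collision capsules.
; Tick turns thumb-index overlaps into laser toggles and clicks, scaling and fading lasers by fingertip distance.
; Clicks or pinch-strength input trigger a mesh swap on a HandPossessor overlapping the right laser.
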(event `InputAxisKey|OculusHand_Left_IndexPinchStrength`
  (params (AxisValue :type "Float (single-precision)"))
  ;[1 1 1] Pinch Events
  (if (or (> AxisValue 0.0) (> (stale `InputAxisKey|OculusHand_Right_IndexPinchStrength` AxisValue) 0.0)) :!label _label
    ;[0 1 0.4658] Example Custom Fire Event
    (bind _ashand_possessor (cast `/Game/HTAB/demo/HandPossessor` (`|GetArrayItem` (`PrimitiveComponent.GetOverlappingActors` (`self.LaserPointer_R`) "/Game/HTAB/demo/HandPossessor.HandPossessor_C")) :!label _label_2))
    (`/Game/HTAB/demo/HandPossessor.MeshSwapLaserFired` _ashand_possessor self)
    (`KismetSystemLibrary.Delay` 0.2)))

(event `self.ReceiveBeginPlay`
  ;[1 1 1] show lasers by default for UE4 Hands, due to bone limitations
  (`KismetSystemLibrary.Delay` 1.0)
  (switch `/Game/HTAB/meshes/HandSkeleton_Type` (`self.HandSkeletonType`)
    (:`NewEnumerator0`
      (`SceneComponent.SetHiddenInGame` (`self.LaserPointer_R`) false false))))

(event `InputAxisKey|OculusHand_Right_IndexPinchStrength`
  (params (AxisValue :type "Float (single-precision)"))
  ;[1 1 1] Pinch Events
  (goto _label))

(event `FireCustomEvent`
  ;[0 1 0.4658] Example Custom Fire Event
  (goto _label_2))

(event `TrackedRHandClickEvent`
  (bind _rspline_dyn (`self.RSpline_Dyn`))
  ;[0 1 0.837] Laser Pointer Clicks
  (`GameplayStatics.PlaySound2D` "/Game/HTAB/blueprints/LaserPointerAssets/click_sound_01B.click_sound_01B" 1.0 1.0 0.0 null null)
  (`MaterialInstanceDynamic.SetVectorParameterValue` _rspline_dyn "LaserColor" (`self.LaserClickColor`))
  (`KismetSystemLibrary.Delay` 0.2)
  (`MaterialInstanceDynamic.SetVectorParameterValue` _rspline_dyn "LaserColor" (`self.LaserHoverColor`))
  (`self.FireCustomEvent`) ; This is whatever logic you want
)

(event `TrackedRHandUnclickEvent`
  ;[0 1 0.837] Laser Pointer Clicks
)

(event `TrackedLHandClickEvent`
  (bind _lspline_dyn (`self.LSpline_Dyn`))
  ;[0 1 0.837] Laser Pointer Clicks
  (`GameplayStatics.PlaySound2D` "/Game/HTAB/blueprints/LaserPointerAssets/click_sound_01B.click_sound_01B" 1.0 1.0 0.0 null null)
  (`MaterialInstanceDynamic.SetVectorParameterValue` _lspline_dyn "LaserColor" (`self.LaserClickColor`))
  (`KismetSystemLibrary.Delay` 0.2)
  (`MaterialInstanceDynamic.SetVectorParameterValue` _lspline_dyn "LaserColor" (`self.LaserHoverColor`))
  (`self.FireCustomEvent`) ; This is whatever logic you want
)

(event `TrackedLHandUnclickEvent`
  ;[0 1 0.837] Laser Pointer Clicks
)

(event `self.ReceiveTick`
  (params (DeltaSeconds :type "Float (single-precision)"))
  (bind _laserinteraction_r (`self.LaserInteraction_R`))
  (bind _laserinteraction_l (`self.LaserInteraction_L`))
  (bind _laserpointer_r (`self.LaserPointer_R`))
  (bind _laserpointer_l (`self.LaserPointer_L`))
  (bind _returnvalue (`KismetMathLibrary.Vector_Distance` (`SceneComponent.K2_GetComponentLocation` (`self.Index_tip_r_click`)) (`SceneComponent.K2_GetComponentLocation` (`self.thumb_tip_r_click`))))
  (bind _returnvalue_2 (`KismetMathLibrary.Vector_Distance` (`SceneComponent.K2_GetComponentLocation` (`self.Index_tip_l_click`)) (`SceneComponent.K2_GetComponentLocation` (`self.thumb_tip_l_click`))))
  (bind _returnvalue_3 (`KismetMathLibrary.MapRangeClamped` _returnvalue 1.0 5.0 0.005 0.075))
  (bind _returnvalue_4 (`KismetMathLibrary.MapRangeClamped` _returnvalue_2 1.0 5.0 0.005 0.075))
  (`|ExecutionSequence`
    (:`then_0`
      ;[1 1 1] Detect if Laser Should be Active
      (if (`PrimitiveComponent.IsOverlappingComponent` (`self.Index_tip_l`) (`self.thumb_tip_l`))
        (`/Engine/EditorBlueprintResources/StandardMacros.DoOnce` false :!label _label_3
          (:`Completed`
            (set `self.isLLaserActive` true)
            (`SceneComponent.SetHiddenInGame` _laserpointer_l false false)
            (`ActorComponent.Activate` _laserinteraction_l false)
            (goto _label_4 :!via `Reset`)))
        (else
          (`|ExecutionSequence`
            (:`then_0`
              (goto _label_3 :!via `Reset`))
            (:`then_1`
              (`/Engine/EditorBlueprintResources/StandardMacros.DoOnce` false :!label _label_4
                (:`Completed`
                  (set `self.isLLaserActive` false)
                  (`SceneComponent.SetHiddenInGame` _laserpointer_l true false)
                  (`ActorComponent.Deactivate` _laserinteraction_l))))))))
    (:`then_1`
      (if (`PrimitiveComponent.IsOverlappingComponent` (`self.Index_tip_r`) (`self.thumb_tip_r`))
        (`/Engine/EditorBlueprintResources/StandardMacros.DoOnce` false :!label _label_5
          (:`Completed`
            (set `self.isRLaserActive` true)
            (`SceneComponent.SetHiddenInGame` _laserpointer_r false false)
            (`ActorComponent.Activate` _laserinteraction_r false)
            (goto _label_6 :!via `Reset`)))
        (else
          (`|ExecutionSequence`
            (:`then_0`
              (goto _label_5 :!via `Reset`))
            (:`then_1`
              (`/Engine/EditorBlueprintResources/StandardMacros.DoOnce` false :!label _label_6
                (:`Completed`
                  (set `self.isRLaserActive` false)
                  (`SceneComponent.SetHiddenInGame` _laserpointer_r true false)
                  (`ActorComponent.Deactivate` _laserinteraction_r))))))))
    (:`then_2`
      ;[1 1 1] Register Finger Click Events
      (if (`PrimitiveComponent.IsOverlappingComponent` (`self.thumb_tip_r_click`) (`self.Index_tip_r_click`))
        (`/Engine/EditorBlueprintResources/StandardMacros.DoOnce` false :!label _label_7
          (:`Completed`
            (`self.TrackedRHandClickEvent`)
            (goto _label_8 :!via `Reset`)))
        (else
          (`|ExecutionSequence`
            (:`then_0`
              (goto _label_7 :!via `Reset`))
            (:`then_1`
              (`/Engine/EditorBlueprintResources/StandardMacros.DoOnce` false :!label _label_8
                (:`Completed`
                  (`self.TrackedRHandUnclickEvent`))))))))
    (:`then_3`
      (if (`PrimitiveComponent.IsOverlappingComponent` (`self.thumb_tip_l_click`) (`self.Index_tip_l_click`))
        (`/Engine/EditorBlueprintResources/StandardMacros.DoOnce` false :!label _label_9
          (:`Completed`
            (`self.TrackedLHandClickEvent`)
            (goto _label_10 :!via `Reset`)))
        (else
          (`|ExecutionSequence`
            (:`then_0`
              (goto _label_9 :!via `Reset`))
            (:`then_1`
              (`/Engine/EditorBlueprintResources/StandardMacros.DoOnce` false :!label _label_10
                (:`Completed`
                  (`self.TrackedLHandUnclickEvent`))))))))
    (:`then_4`
      ;[1 1 1] Laser Dynamic Parameters
      (if (and (`self.isRLaserActive`) (`self.isRLaserEnabled`))
        (`SceneComponent.SetRelativeScale3D` (`self.LaserPointer_R`) (`KismetMathLibrary.MakeVector` _returnvalue_3 _returnvalue_3 (`KismetMathLibrary.MapRangeClamped` _returnvalue 1.0 5.0 1.0 0.001)))
        (`MaterialInstanceDynamic.SetScalarParameterValue` (`self.RSpline_Dyn`) "Opacity" (`KismetMathLibrary.MapRangeClamped` _returnvalue 1.0 3.0 0.05))))
    (:`then_5`
      (if (and (`self.isLLaserEnabled`) (`self.isLLaserEnabled`))
        (`SceneComponent.SetRelativeScale3D` (`self.LaserPointer_L`) (`KismetMathLibrary.MakeVector` _returnvalue_4 _returnvalue_4 (`KismetMathLibrary.MapRangeClamped` _returnvalue_2 1.0 5.0 1.0 0.001)))
        (`MaterialInstanceDynamic.SetScalarParameterValue` (`self.LSpline_Dyn`) "Opacity" (`KismetMathLibrary.MapRangeClamped` _returnvalue_2 1.0 3.0 0.05))))))

(fn `PositionCapsules`
  (params (BoneNamesArray :type "Array of Name") (CapsuleCollArray :type "Array of CapsuleComponent Object Reference") (OculusHand :type "OculusHandComponent Object Reference"))
  (`KismetArrayLibrary.Array_Clear` CapsuleCollArray)
  (for _array_element BoneNamesArray
    (bind _returnvalue_location (`KismetMathLibrary.BreakTransform` (`SceneComponent.GetSocketTransform` OculusHand (`SkinnedMeshComponent.GetParentBone` OculusHand _array_element) "RTS_Actor")))
    (bind _returnvalue (`SceneComponent.GetSocketTransform` OculusHand _array_element "RTS_Actor"))
    (bind _returnvalue_2 (`AddComponent|NODE_AddCapsuleComponent-0` :`bManualAttachment` true :`RelativeTransform` (`KismetMathLibrary.MakeTransform` (+ _returnvalue_location (/ (- (.location _returnvalue) _returnvalue_location) 2.8)) (`KismetMathLibrary.ComposeRotators` (struct :`Pitch` 90.0) (.rotation _returnvalue)))))
    (`KismetArrayLibrary.Array_Add` CapsuleCollArray _returnvalue_2)
    (`CapsuleComponent.SetCapsuleRadius` _returnvalue_2 (* (.x (.scale _returnvalue)) 0.8) true)
    (`CapsuleComponent.SetCapsuleHalfHeight` _returnvalue_2 (* (/ (`KismetMathLibrary.VSize` (- _returnvalue_location (.location _returnvalue))) 2.0) 0.5) true)
    (`PrimitiveComponent.SetCollisionEnabled` _returnvalue_2 "QueryAndPhysics")
    (`PrimitiveComponent.SetCollisionResponseToAllChannels` _returnvalue_2 "ECR_Block")
    (`SceneComponent.K2_AttachToComponent` _returnvalue_2 OculusHand _array_element "SnapToTarget" "KeepWorld" "SnapToTarget" true)))

(fn `UserConstructionScript`
  (`|ExecutionSequence`
    (:`then_0`
      (switch `/Game/HTAB/meshes/HandSkeleton_Type` (`self.HandSkeletonType`)
        (:`NewEnumerator0`
          (`self.PositionCapsules` (`self.BoneNamesUE4_L`) (`self.CapsuleCols_L`) (`self.OculusHand_L_UE4`))
          (`self.PositionCapsules` (`self.BoneNamesUE4_R`) (`self.CapsuleCols_R`) (`self.OculusHand_R_UE4`))
          (`SceneComponent.K2_AttachToComponent` (`self.thumb_tip_l`) (`self.OculusHand_L_UE4`) "thumb_03_l" "KeepRelative" "SnapToTarget" "KeepRelative" true)
          (`SceneComponent.K2_AttachToComponent` (`self.Index_tip_l`) (`self.OculusHand_L_UE4`) "index_03_l" "KeepRelative" "SnapToTarget" "KeepRelative" true)
          (`SceneComponent.K2_AttachToComponent` (`self.Index_tip_r`) (`self.OculusHand_R_UE4`) "index_03_r" "KeepRelative" "SnapToTarget" "KeepRelative" true)
          (`SceneComponent.K2_AttachToComponent` (`self.thumb_tip_r`) (`self.OculusHand_R_UE4`) "thumb_03_r" "KeepRelative" "SnapToTarget" "KeepRelative" true)
          (`SceneComponent.K2_AttachToComponent` (`self.LaserPointer_R`) (`self.OculusHand_R_UE4`) "hand_rSocket" "SnapToTarget" "SnapToTarget" "KeepWorld" true)
          (`SceneComponent.K2_AttachToComponent` (`self.LaserPointer_L`) (`self.OculusHand_L_UE4`) "hand_lSocket" "SnapToTarget" "SnapToTarget" "KeepWorld" true)
          (`SceneComponent.K2_AttachToComponent` (`self.Index_tip_r_click`) (`self.OculusHand_R_UE4`) "index_03_r" "KeepRelative" "SnapToTarget" "KeepRelative" true)
          (`SceneComponent.K2_AttachToComponent` (`self.thumb_tip_r_click`) (`self.OculusHand_R_UE4`) "thumb_03_r" "KeepRelative" "SnapToTarget" "KeepRelative" true)
          (`SceneComponent.K2_AttachToComponent` (`self.Index_tip_l_click`) (`self.OculusHand_L_UE4`) "index_03_l" "KeepRelative" "SnapToTarget" "KeepRelative" true)
          (`SceneComponent.K2_AttachToComponent` (`self.thumb_tip_l_click`) (`self.OculusHand_L_UE4`) "thumb_03_l" "KeepRelative" "SnapToTarget" "KeepRelative" true)
          (`SceneComponent.K2_AttachToComponent` (`self.WidgetInteraction_L_UE4`) (`self.OculusHand_L_UE4`) "index_03_l" "KeepRelative" "KeepRelative" "KeepRelative" true)
          (`SceneComponent.K2_AttachToComponent` (`self.WidgetInteraction_R_UE4`) (`self.OculusHand_R_UE4`) "index_03_r" "KeepRelative" "KeepRelative" "KeepRelative" true)
          ;[0.503 1 0.7265] Remove unused Hand Components
          (`ActorComponent.K2_DestroyComponent` (`self.OculusHand_R_Oc`))
          (`ActorComponent.K2_DestroyComponent` (`self.OculusHand_L_Oc`))
          (`ActorComponent.K2_DestroyComponent` (`self.WidgetInteraction_R_Oc`))
          (`ActorComponent.K2_DestroyComponent` (`self.WidgetInteraction_L_Oc`)))
        (:`NewEnumerator1`
          (`self.PositionCapsules` (`self.BoneNamesOculus_L`) (`self.CapsuleCols_L`) (`self.OculusHand_L_Oc`))
          (`self.PositionCapsules` (`self.BoneNamesOculus_R`) (`self.CapsuleCols_R`) (`self.OculusHand_R_Oc`))
          (`SceneComponent.K2_AttachToComponent` (`self.thumb_tip_l`) (`self.OculusHand_L_Oc`) "b_l_thumb3" "KeepRelative" "SnapToTarget" "KeepRelative" true)
          (`SceneComponent.K2_AttachToComponent` (`self.Index_tip_l`) (`self.OculusHand_L_Oc`) "b_l_index3" "KeepRelative" "SnapToTarget" "KeepRelative" true)
          (`SceneComponent.K2_AttachToComponent` (`self.Index_tip_r`) (`self.OculusHand_R_Oc`) "b_r_index3" "KeepRelative" "SnapToTarget" "KeepRelative" true)
          (`SceneComponent.K2_AttachToComponent` (`self.thumb_tip_r`) (`self.OculusHand_R_Oc`) "b_r_thumb3" "KeepRelative" "SnapToTarget" "KeepRelative" true)
          (`SceneComponent.K2_AttachToComponent` (`self.LaserPointer_R`) (`self.OculusHand_R_Oc`) "b_r_wrist" "KeepRelative" "KeepRelative" "KeepRelative" true)
          (`SceneComponent.K2_AttachToComponent` (`self.LaserPointer_L`) (`self.OculusHand_L_Oc`) "b_l_wrist" "KeepRelative" "KeepRelative" "KeepRelative" true)
          (`SceneComponent.K2_AttachToComponent` (`self.Index_tip_r_click`) (`self.OculusHand_R_Oc`) "b_r_index3" "KeepRelative" "SnapToTarget" "KeepRelative" true)
          (`SceneComponent.K2_AttachToComponent` (`self.thumb_tip_r_click`) (`self.OculusHand_R_Oc`) "b_r_thumb3" "KeepRelative" "SnapToTarget" "KeepRelative" true)
          (`SceneComponent.K2_AttachToComponent` (`self.Index_tip_l_click`) (`self.OculusHand_L_Oc`) "b_l_index3" "KeepRelative" "SnapToTarget" "KeepRelative" true)
          (`SceneComponent.K2_AttachToComponent` (`self.thumb_tip_l_click`) (`self.OculusHand_L_Oc`) "b_l_thumb3" "KeepRelative" "SnapToTarget" "KeepRelative" true)
          (`SceneComponent.K2_AttachToComponent` (`self.WidgetInteraction_L_Oc`) (`self.OculusHand_L_Oc`) "b_l_index3" "KeepRelative" "KeepRelative" "KeepRelative" true)
          (`SceneComponent.K2_AttachToComponent` (`self.WidgetInteraction_R_Oc`) (`self.OculusHand_R_Oc`) "b_r_index3" "KeepRelative" "KeepRelative" "KeepRelative" true)
          (`ActorComponent.K2_DestroyComponent` (`self.OculusHand_R_UE4`))
          (`ActorComponent.K2_DestroyComponent` (`self.WidgetInteraction_R_UE4`))
          (`ActorComponent.K2_DestroyComponent` (`self.OculusHand_L_UE4`))
          (`ActorComponent.K2_DestroyComponent` (`self.WidgetInteraction_L_UE4`)))))
    (:`then_1`
      ;[1 1 1] Init Laser Dynamic Materials
      (bind _returnvalue (`KismetMaterialLibrary.CreateDynamicMaterialInstance` (`PrimitiveComponent.GetMaterial` (`self.LaserPointer_R`) 0)))
      (bind _output_get (set `self.RSpline_Dyn` _returnvalue))
      (`PrimitiveComponent.SetMaterialByName` (`self.LaserPointer_R`) "LaserMat" _output_get))
    (:`then_2`
      (bind _returnvalue_2 (`KismetMaterialLibrary.CreateDynamicMaterialInstance` (`PrimitiveComponent.GetMaterial` (`self.LaserPointer_L`) 0)))
      (bind _output_get_2 (set `self.LSpline_Dyn` _returnvalue_2))
      (`PrimitiveComponent.SetMaterialByName` (`self.LaserPointer_L`) "LaserMat" _output_get_2))))