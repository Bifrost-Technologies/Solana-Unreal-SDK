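; MetaplexTerminal is an in-world terminal actor that links nearby players to a Metaplex minting screen.
; Its trigger registers the terminal on the character's PlayerController and sets that controller as the Loginscreen widget's MachineUser.
; Leaving clears NearbyTerminal but still sets IsNearMetaplexMachine to true.
; AI Perception updates show a text render for five seconds, or hide it when no actors are reported.
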(event `self.ReceiveBeginPlay`
  (add `AIPerceptionComponent.OnPerceptionUpdated` (`self.AIPerception`) (delegate `OnPerceptionUpdated_Event`)))

(event `OnPerceptionUpdated_Event`
  (params (UpdatedActors :type "Array of Actor Object Reference (by ref)"))
  (bind _textrender (`self.TextRender`))
  (if (!= (`KismetArrayLibrary.Array_Length` UpdatedActors) 0)
    (`SceneComponent.SetVisibility` _textrender true false)
    (`KismetSystemLibrary.Delay` 5.0)
    (`SceneComponent.SetVisibility` _textrender false false)
    (else
      (`SceneComponent.SetVisibility` (`self.TextRender`) false false))))

(event `self.ReceiveTick`
  (params (DeltaSeconds :type "Float (single-precision)")))

(event `self.Trigger.OnComponentBeginOverlap`
  (params (OverlappedComponent :type "PrimitiveComponent Object Reference") (OtherActor :type "Actor Object Reference") (OtherComp :type "PrimitiveComponent Object Reference") (OtherBodyIndex :type Integer) (bFromSweep :type Boolean) (SweepResult :type "HitResult Structure (by ref)"))
  (bind _asbp_third_person_character (cast `/Game/ThirdPerson/Blueprints/BP_ThirdPersonCharacter` OtherActor))
  (bind _playercontroller (`/Game/ThirdPerson/Blueprints/BP_ThirdPersonCharacter.PlayerController` _asbp_third_person_character))
  (set `/Game/ThirdPerson/Blueprints/SolanaPlayerController.isNearMetaplexMachine` true _playercontroller)
  (set `/Game/ThirdPerson/Blueprints/SolanaPlayerController.NearbyTerminal` self _playercontroller)
  (bind _asmetaplex_minting_widget (cast `/Game/MetaplexStore/blueprint/MetaplexMintingWidget` (`WidgetComponent.GetWidget` (`self.loginscreen`))))
  (set `/Game/MetaplexStore/blueprint/MetaplexMintingWidget.MachineUser` _playercontroller _asmetaplex_minting_widget))

(event `self.Trigger.OnComponentEndOverlap`
  (params (OverlappedComponent :type "PrimitiveComponent Object Reference") (OtherActor :type "Actor Object Reference") (OtherComp :type "PrimitiveComponent Object Reference") (OtherBodyIndex :type Integer))
  (bind _asbp_third_person_character (cast `/Game/ThirdPerson/Blueprints/BP_ThirdPersonCharacter` OtherActor))
  (bind _playercontroller (`/Game/ThirdPerson/Blueprints/BP_ThirdPersonCharacter.PlayerController` _asbp_third_person_character))
  (set `/Game/ThirdPerson/Blueprints/SolanaPlayerController.isNearMetaplexMachine` true _playercontroller)
  (set `/Game/ThirdPerson/Blueprints/SolanaPlayerController.NearbyTerminal` null _playercontroller))

(fn `UserConstructionScript`)