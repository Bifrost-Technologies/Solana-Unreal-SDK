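; TcpComponent is a TCP socket actor in the MetaplexStore content that requests a signature for a transaction message from a local Tranquility service.
; On BeginPlay it stores itself in LinkStream, and ConnectToLinkStream opens a localhost connection.
; Once connected it sends a pipe-delimited RequestSignature request carrying the transaction message.
; Any response is only printed on screen, and disconnection is left unhandled.
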(event `ConnectToLinkStream`
  (params (TransactionMessage :type String))
  (`self.Connect` "127.0.0.1" 50505 (delegate `Disconnected`) (delegate `Connected`) (delegate `MessageReceived`)))

(event `Connected`
  (params (ConnectionId :type Integer))
  (`KismetSystemLibrary.PrintString` "Connected to Tranquility!" true true (struct :`G` 0.66 :`B` 1.0 :`A` 1.0) 1.0)
  (`self.SendData` ConnectionId (`self.Conv_StringToBytes` (`KismetStringLibrary.JoinStringArray` (`|MakeArray` "RequestSignature" (stale `ConnectToLinkStream` TransactionMessage)) "|"))))

(event `self.ReceiveBeginPlay`
  (set `self.Link Stream` self))

(event `MessageReceived`
  (params (ConnectionId :type Integer) (Message :type "Array of Byte (by ref)"))
  (`KismetSystemLibrary.PrintString` "Response received")
  (bind _returnvalue (`self.Message_ReadString` Message 1000))
  (`KismetSystemLibrary.PrintString` _returnvalue true true (struct :`G` 0.66 :`B` 1.0 :`A` 1.0) 10.0))

(event `Disconnected`
  (params (ConnectionId :type Integer)))

(fn `UserConstructionScript`)