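; Automatic double sliding apartment door that opens when something overlaps its Box trigger and closes when the overlap ends.
; Two static mesh panels slide apart in opposite directions along the local Y axis using MoveComponentTo, then return to their relative origin on exit.
; The second panel keeps a half-turn rotation in both moves.
; Overlaps are not filtered by actor or counted.
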(event `self.Box.OnComponentBeginOverlap`
  (params (OverlappedComponent :type "PrimitiveComponent Object Reference") (OtherActor :type "Actor Object Reference") (OtherComp :type "PrimitiveComponent Object Reference") (OtherBodyIndex :type Integer) (bFromSweep :type Boolean) (SweepResult :type "HitResult Structure (by ref)"))
  (`|ExecutionSequence`
    (:`then_0`
      (`KismetSystemLibrary.MoveComponentTo` (`self.StaticMesh`) (0.0 -100.0 0.0) (struct) false false 0.5))
    (:`then_1`
      (`KismetSystemLibrary.MoveComponentTo` (`self.StaticMesh1`) (0.0 100.0 0.0) (struct :`Yaw` 180.0) false false 0.5))))

(event `self.Box.OnComponentEndOverlap`
  (params (OverlappedComponent :type "PrimitiveComponent Object Reference") (OtherActor :type "Actor Object Reference") (OtherComp :type "PrimitiveComponent Object Reference") (OtherBodyIndex :type Integer))
  (`|ExecutionSequence`
    (:`then_0`
      (`KismetSystemLibrary.MoveComponentTo` (`self.StaticMesh`) (0.0 0.0 0.0) (struct) false false 0.5))
    (:`then_1`
      (`KismetSystemLibrary.MoveComponentTo` (`self.StaticMesh1`) (0.0 0.0 0.0) (struct :`Yaw` 180.0) false false 0.5))))

(fn `UserConstructionScript`)